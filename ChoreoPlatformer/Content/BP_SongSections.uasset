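; BP_SongSections drives the song audio of a rhythm dance game by sending parameters and triggers to an audio component.
; It starts the song when controller calibration ends and sends a trigger on each new tempo from the song tempo component.
; Playing a section sets its wave, start point and BPM, then fades intro volume with a timeline.
; Tempo results set execution pitch by grade and success rate from the dancer's health accuracy.
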(event `self.ReceiveBeginPlay`
  (set `self.DancerHealth` (`self.GetComponentByClass` (`GameplayStatics.GetPlayerController` 0) "/Script/ChoreoPlatformer.DancerHealthComponent"))
  (add `SongTempoComponent.NewTempoStarted` (`DanceUtilsFunctionLibrary.GetSongTempoComponent`) (delegate `MarkTempo`))
  (bind _aschoreo_player_controller (cast `ChoreoPlayerController` (`GameplayStatics.GetPlayerController` 0)))
  (add `ChoreoPlayerController.CalibrationEnded` _aschoreo_player_controller (delegate `CalibrationEnded`)))

(event `CalibrationEnded`
  (`AudioParameterControllerInterface.SetTriggerParameter` (`self.Audio`) "StartSong"))

(event `MarkTempo`
  (`AudioParameterControllerInterface.SetTriggerParameter` (`self.Audio`) "TempoStarted"))

(event `self.PlayCurrentSection`
  (`self.SetupCurrentSection`)
  (`AudioParameterControllerInterface.SetTriggerParameter` (`self.Audio`) "NewSection")
  (bind (_direction _volume) (`Timeline|MusicFade` :!via `PlayFromStart`)
    (:`Update`
      (`AudioParameterControllerInterface.SetFloatParameter` (`self.Audio`) "IntroVolume" _volume))))

(event `self.PlayTempoResult`
  (params (Result :type "ETempoAccuracy Enum" :default "Bad"))
  (`AudioParameterControllerInterface.SetFloatParameter` (`self.Audio`) "ExecutionPitch" (`self.GetResultPitch` Result))
  (`AudioParameterControllerInterface.SetFloatParameter` (`self.Audio`) "SuccessRate" (`DancerHealthComponent.GetCurrentAccuracy` (`self.DancerHealth`)))
  (`AudioParameterControllerInterface.SetTriggerParameter` (`self.Audio`) "TempoExecuted"))

(fn `GetResultPitch`
  (params (Accuracy :type "ETempoAccuracy Enum" :default "Bad"))
  (returns (Pitch :type "Float (double-precision)"))
  (switch `ETempoAccuracy` Accuracy
    (:`Bad`
      (return -5.0))
    (:`Great`
      (return -1.0))
    (:`Perfect`
      (return 0.0))))

(fn `SetupCurrentSection`
  (bind _audio (`self.Audio`))
  (`|ExecutionSequence`
    (:`then_0`
      (`AudioParameterControllerInterface.SetFloatParameter` (`self.Audio`) "CurrentSectionStart" (`self.CurrentSectionStart`)))
    (:`then_1`
      (`AudioComponent.SetWaveParameter` _audio "Song" (`self.SectionSong`)))
    (:`then_2`
      (`AudioParameterControllerInterface.SetFloatParameter` _audio "SongBPM" (`self.CurrentSongBPM`)))))

(fn `UserConstructionScript`)