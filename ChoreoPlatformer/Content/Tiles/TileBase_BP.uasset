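; Base tile Blueprint for a music-themed game, drawn as a sprite chosen by its tile type, such as Black, Half, Blocker or a directional Force.
; PaintTile sets the sprite from GetTileSprite and creates a dynamic M_Tile material instance on it.
; Each Tick drives that material's LightMultiplier parameter from SongTempo's result, so the tile's lighting follows the song's tempo.
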(event `self.PaintTile`
  (`PaperSpriteComponent.SetSprite` (`self.Sprite`) (`self.GetTileSprite`))
  (bind _returnvalue (`PrimitiveComponent.CreateDynamicMaterialInstance` (`self.Sprite`) 0 "/Game/CityBuilding/Materials/M_Tile.M_Tile" "None"))
  (set `self.TileMat` _returnvalue))

(event `self.ReceiveTick`
  (params (DeltaSeconds :type "Float (single-precision)"))
  (`MaterialInstanceDynamic.SetVectorParameterValue` (`self.TileMat`) "LightMultiplier" (`KismetMathLibrary.Conv_DoubleToLinearColor` (* (`SongTempoComponent.TempoResult` (`self.SongTempo`) 1.0) 1.5))))

(fn `GetTileSprite`
  (returns (TileSprite :type "PaperSprite Object Reference"))
  (switch `ETempoTile` (`self.TileType`)
    (:`Black`
      (return "/Game/Tiles/notes_Sprite.notes_Sprite"))
    (:`Half`
      (return "/Game/Tiles/notes_Sprite2.notes_Sprite2"))
    (:`Blocker`
      (return "/Game/Tiles/notes_Sprite1.notes_Sprite1"))
    (:`ForceUp`
      (return "/Game/Tiles/notes_Sprite3.notes_Sprite3"))
    (:`ForceDown`
      (return "/Game/Tiles/notes_Sprite4.notes_Sprite4"))
    (:`ForceLeft`
      (return "/Game/Tiles/notes_Sprite5.notes_Sprite5"))
    (:`ForceRight`
      (return "/Game/Tiles/notes_Sprite6.notes_Sprite6"))))

(fn `UserConstructionScript`)