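; Walking enemy Blueprint for a tile-based game, handling the visuals and sound of each move.
; On BeginPlay it sets the mesh's custom depth stencil and creates a dynamic citizen material, stored as ShineMat, with its light multiplier at zero.
; Each StartedWalking event plays the movement animation once, flipping the mesh's X scale on alternate moves to mirror it.
; The step sound plays in 2D, with volume scaled manually by tile distance from the player.
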(event `self.ReceiveBeginPlay`
  (`PrimitiveComponent.SetCustomDepthStencilValue` (`self.Mesh`) 2)
  (bind _returnvalue (`PrimitiveComponent.CreateDynamicMaterialInstance` (`self.Mesh`) 0 "/Game/Enemies/Meshes/M_Citizen.M_Citizen" "None"))
  (bind _output_get (set `self.ShineMat` _returnvalue))
  (`MaterialInstanceDynamic.SetScalarParameterValue` _output_get "LightMultiplier" 0.0))

(event `self.StartedWalking`
  (`SceneComponent.SetRelativeScale3D` (`self.Mesh`) (`KismetMathLibrary.MakeVector` (`self.ShouldMirror`) 1.0 1.0))
  (`SkeletalMeshComponent.PlayAnimation` (`self.Mesh`) (`self.Movement Animation`) false)
  (set `self.ShouldMirror` (* (`self.ShouldMirror`) -1.0))
  (`GameplayStatics.PlaySound2D` "/Game/Sounds/enemy_step.enemy_step" (/ (- 5 (`DanceUtilsFunctionLibrary.TilesAwayFromPlayer`)) 5.0) 1.0 0.0 null null false))

(fn `UserConstructionScript`)