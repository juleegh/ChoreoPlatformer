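; Enemy Blueprint that handles the animation and sound feedback when a forward enemy starts walking on a tile-based map.
; Each step plays the movement animation once and flips the ShouldMirror sign, so the mesh's X scale mirrors on alternate steps from a single animation.
; A 2D step sound fakes distance attenuation by scaling its volume down linearly with the tile distance to the player.
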(event `self.StartedWalking`
  (`SceneComponent.SetRelativeScale3D` (`self.Mesh`) (`KismetMathLibrary.MakeVector` (`self.ShouldMirror`) 1.0 1.0))
  (`SkeletalMeshComponent.PlayAnimation` (`self.Mesh`) (`self.Movement Animation`) false)
  (set `self.ShouldMirror` (* (`self.ShouldMirror`) -1.0))
  (`GameplayStatics.PlaySound2D` "/Game/Sounds/enemy_step.enemy_step" (/ (- 5 (`DanceUtilsFunctionLibrary.TilesAwayFromPlayer`)) 5.0) 1.0 0.0 null null false))

(fn `UserConstructionScript`)