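; Base Blueprint for a neon sign that alternates between two light colors in time with the song tempo.
; On BeginPlay it creates a dynamic material on its static mesh, applies the MainLight and SecondLight colors, and binds to the song tempo component's new-tempo event.
; Each tempo event flips a boolean to swap the two colors between the material's vector parameters.
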(event `self.ReceiveBeginPlay`
  (bind _staticmesh (`self.StaticMesh`))
  (add `SongTempoComponent.NewTempoStarted` (`ComponentGettersFunctionLibrary.GetSongTempoComponent`) (delegate `TempoBeat`))
  (bind _returnvalue (`PrimitiveComponent.CreateDynamicMaterialInstance` _staticmesh 0 (`PrimitiveComponent.GetMaterial` _staticmesh 0) "None"))
  (bind _output_get (set `self.NeonMaterial` _returnvalue))
  (`MaterialInstanceDynamic.SetVectorParameterValue` _output_get "MainLight" (`self.MainLight`))
  (`MaterialInstanceDynamic.SetVectorParameterValue` _output_get "SecondLight" (`self.SecondLight`)))

(event `TempoBeat`
  (if (`self.IsOnFirst`)
    (`MaterialInstanceDynamic.SetVectorParameterValue` (`self.NeonMaterial`) "MainLight" (`self.SecondLight`))
    (`MaterialInstanceDynamic.SetVectorParameterValue` (`self.NeonMaterial`) "SecondLight" (`self.MainLight`))
    (else
      (`MaterialInstanceDynamic.SetVectorParameterValue` (`self.NeonMaterial`) "MainLight" (`self.MainLight`))
      (`MaterialInstanceDynamic.SetVectorParameterValue` (`self.NeonMaterial`) "SecondLight" (`self.SecondLight`))))
  (set `self.IsOnFirst` (not (`self.IsOnFirst`))))

(fn `UserConstructionScript`)