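; Base Blueprint for luminous city-building assets that twinkle in time with the song tempo.
; On BeginPlay it binds to the choreo controller's tempo component, tints the point light and creates a dynamic mesh material with the same color.
; Each tempo event restarts the Twinkle timeline, whose intensity curve drives both the light's intensity and the material's light multiplier.
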(event `self.ReceiveBeginPlay`
  (bind _asbp_choreo_controller (cast `/Game/BP_ChoreoController` (`GameplayStatics.GetPlayerController` 0)))
  (add `SongTempoComponent.NewTempoStarted` (`ChoreoPlayerController.GetSongTempoComponent` _asbp_choreo_controller) (delegate `TempoBeat`))
  (`LightComponent.SetLightColor` (`self.PointLight`) (`self.LightColor`) true)
  (bind _returnvalue (`PrimitiveComponent.CreateDynamicMaterialInstance` (`self.StaticMesh`) 0 "/Game/CityBuilding/Materials/Luminous/L_Material.L_Material" "None"))
  (bind _output_get (set `self.LightMaterial` _returnvalue))
  (`MaterialInstanceDynamic.SetVectorParameterValue` _output_get "Light" (`self.LightColor`)))

(event `TempoBeat`
  (bind (_direction _intensity) (`Timeline|Twinkle` :!via `PlayFromStart`)
    (:`Update`
      (`LightComponent.SetIntensity` (`self.PointLight`) (* _intensity (`self.LightIntensity`)))
      (`MaterialInstanceDynamic.SetVectorParameterValue` (`self.LightMaterial`) "LightMultiplier" (`KismetMathLibrary.Conv_DoubleToLinearColor` _intensity)))))

(fn `UserConstructionScript`)