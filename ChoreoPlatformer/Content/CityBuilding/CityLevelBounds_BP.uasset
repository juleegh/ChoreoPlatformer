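; City level bounds actor that forms a rectangular boundary from four side components: North, South, East and West.
; The construction script scales and offsets each side from Width, Depth and Height, keeping a fixed thickness and centering the rectangle on the actor.
; It has no runtime logic, as the event graph holds only disabled default events.
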(fn `UserConstructionScript`
  (bind _south (`self.South`))
  (bind _west (`self.West`))
  (bind _east (`self.East`))
  (bind _north (`self.North`))
  (`|ExecutionSequence`
    (:`then_0`
      (`SceneComponent.SetRelativeScale3D` _north (`KismetMathLibrary.MakeVector` (`self.Width`) 50.0 (`self.Height`)))
      (`SceneComponent.K2_SetRelativeLocation` _north (`KismetMathLibrary.MakeVector` 0.0 (* (`self.Depth`) 1.0)) false false))
    (:`then_1`
      (`SceneComponent.SetRelativeScale3D` _south (`KismetMathLibrary.MakeVector` (`self.Width`) 50.0 (`self.Height`)))
      (`SceneComponent.K2_SetRelativeLocation` _south (`KismetMathLibrary.MakeVector` 0.0 (* (`self.Depth`) -1.0)) false false))
    (:`then_2`
      (`SceneComponent.SetRelativeScale3D` _west (`KismetMathLibrary.MakeVector` 50.0 (`self.Depth`) (`self.Height`)))
      (`SceneComponent.K2_SetRelativeLocation` _west (`KismetMathLibrary.MakeVector` (* (`self.Width`) -1.0)) false false))
    (:`then_3`
      (`SceneComponent.SetRelativeScale3D` _east (`KismetMathLibrary.MakeVector` 50.0 (`self.Depth`) (`self.Height`)))
      (`SceneComponent.K2_SetRelativeLocation` _east (`KismetMathLibrary.MakeVector` (* (`self.Width`) 1.0)) false false))))