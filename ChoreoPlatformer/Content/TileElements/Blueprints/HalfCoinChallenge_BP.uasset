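; Half-coin challenge tile element: two coin halves sit at the first and last points of a spline, with a dialog box showing the remaining tempos above the end one.
; Both coins bounce on each new song tempo through a timeline.
; Challenge start hides the start coin, swaps the end sprite and begins the countdown display.
; Challenge end hides the end coin and dialog, playing a win sound with star particles or a fail sound.
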(event `self.ReceiveBeginPlay`
  (`parent.ReceiveBeginPlay`)
  (`self.SetStartCoin`)
  (`self.SetEndCoin`)
  (`TextRenderComponent.K2_SetText` (`self.RemainingTempos`) (`KismetTextLibrary.Conv_IntToText` (`self.TemposBetweenHalfs`)) :!label _label)
  (add `SongTempoComponent.NewTempoStarted` (`DanceUtilsFunctionLibrary.GetSongTempoComponent`) (delegate `Bounce Coins`)))

(event `self.ChallengeStarted`
  (`PaperSpriteComponent.SetSprite` (`self.EndCoin`) "/Game/Sprites/challenge_assets_Sprite_8.challenge_assets_Sprite_8")
  (`SceneComponent.SetVisibility` (`self.StartCoin`) false false)
  (`GameplayStatics.PlaySound2D` "/Game/Sounds/coin_start.coin_start" 1.0 1.0 0.0 null null)
  (goto _label))

(event `Bounce Coins`
  (bind _startcoin (`self.StartCoin`))
  (bind _endcoin (`self.EndCoin`))
  (bind (_returnvalue_x _returnvalue_y) (`KismetMathLibrary.BreakVector` (`SceneComponent.K2_GetComponentLocation` _startcoin)))
  (bind (_returnvalue_x_2 _returnvalue_y_2) (`KismetMathLibrary.BreakVector` (`SceneComponent.K2_GetComponentLocation` _endcoin)))
  (bind (_direction _height) (`Timeline|Bounce` :!via `PlayFromStart`)
    (:`Update`
      (bind _returnvalue (+ (* _height 10.0) 50.0))
      (`SceneComponent.K2_SetWorldLocation` _startcoin (`KismetMathLibrary.MakeVector` _returnvalue_x _returnvalue_y _returnvalue) false false)
      (`SceneComponent.K2_SetWorldLocation` _endcoin (`KismetMathLibrary.MakeVector` _returnvalue_x_2 _returnvalue_y_2 _returnvalue) false false))))

(event `self.ChallengeEnded`
  (params (bWasSuccessful :type Boolean))
  (`SceneComponent.SetVisibility` (`self.DialogBox`) false true)
  (`SceneComponent.SetVisibility` (`self.EndCoin`) false true)
  (if bWasSuccessful
    (`GameplayStatics.PlaySound2D` "/Game/Sounds/coin_win.coin_win" 1.0 1.0 0.0 null null)
    (`GameplayStatics.SpawnEmitterAtLocation` "/Game/Particles/Stars_PS.Stars_PS" (`SceneComponent.K2_GetComponentLocation` (`self.EndCoin`)))
    (else
      (`GameplayStatics.PlaySound2D` "/Game/Sounds/coin_fail.coin_fail" 1.0 1.0 0.0 null null))))

(event `self.ChallengeUpdated`
  (`TextRenderComponent.K2_SetText` (`self.RemainingTempos`) (`KismetTextLibrary.Conv_IntToText` (`self.TemposRemaining`))))

(fn `SetEndCoin`
  (bind _interestpoints (`self.InterestPoints`))
  (bind _returnvalue (+ (`SplineComponent.GetLocationAtSplinePoint` _interestpoints (- (`SplineComponent.GetNumberOfSplinePoints` _interestpoints) 1) "World") (0.0 0.0 50.0)))
  (`SceneComponent.K2_SetWorldLocation` (`self.EndCoin`) _returnvalue false false)
  (`PaperSpriteComponent.SetSpriteColor` (`self.EndCoin`) (struct :`R` 1.0 :`G` 1.0 :`B` 1.0 :`A` 1.0))
  (`SceneComponent.K2_SetWorldLocation` (`self.DialogBox`) (+ _returnvalue (0.0 0.0 100.0)) false false))

(fn `SetStartCoin`
  (`SceneComponent.K2_SetWorldLocation` (`self.StartCoin`) (+ (`SplineComponent.GetLocationAtSplinePoint` (`self.InterestPoints`) 0 "World") (0.0 0.0 50.0)) false false)
  (`PaperSpriteComponent.SetSpriteColor` (`self.StartCoin`) (struct :`R` 1.0 :`G` 1.0 :`B` 1.0 :`A` 1.0)))

(fn `UserConstructionScript`)