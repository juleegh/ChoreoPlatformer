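; Fruit tile element that shows a paper sprite bobbing vertically above its base.
; A self-restarting timeline drives the sprite's relative Z, with the hover offset scaled by the song tempo component's frequency.
; RefreshState hides the sprite, makes it ignore all collision channels and stops the hover timeline.
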(event `self.ReceiveBeginPlay`
  (bind (_direction _hover) (`Timeline|Timeline_0` :!label _label)
    (:`Update`
      (`SceneComponent.K2_SetRelativeLocation` (`self.PaperSprite`) (`KismetMathLibrary.MakeVector` 0.0 0.0 (+ (* _hover (`SongTempoComponent.GetFrequency` (`DanceUtilsFunctionLibrary.GetSongTempoComponent`)) 10.0) 60.0)) false false))
    (:`Finished`
      (`|ExecutionSequence`
        (:`then_0`
          (goto _label :!via `PlayFromStart`))))))

(event `self.RefreshState`
  (bind _papersprite (`self.PaperSprite`))
  (`SceneComponent.SetVisibility` _papersprite false false)
  (`PrimitiveComponent.SetCollisionResponseToAllChannels` _papersprite "ECR_Ignore")
  (goto _label :!via `Stop`))

(fn `UserConstructionScript`)