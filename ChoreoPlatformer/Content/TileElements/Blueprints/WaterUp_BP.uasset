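; WaterUp tile element with an animated button mesh that pulses in time with the song tempo.
; On BeginPlay it binds to the song tempo component and scales animation rate by the tempo frequency, then replays the idle animation each tempo event while interactable.
; RefreshState only plays the button sound.
; The stop/go sprite swaps and press animation are unconnected, and reset does nothing.
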(event `self.ReceiveBeginPlay`
  (bind _returnvalue (`ComponentGettersFunctionLibrary.GetSongTempoComponent`))
  (add `SongTempoComponent.NewTempoStarted` _returnvalue (delegate `Tempo`))
  (set `SkeletalMeshComponent.GlobalAnimRateScale` (/ 1.0 (`SongTempoComponent.GetFrequency` _returnvalue)) (`self.SkeletalMesh`)))

(event `Tempo`
  (if (`self.CanInteract`)
    (`SkeletalMeshComponent.PlayAnimation` (`self.SkeletalMesh`) "/Game/TileElements/Meshes/Button/button_Anim_Button_Idle.button_Anim_Button_Idle" false)))

(event `self.RefreshState`
  (`GameplayStatics.PlaySound2D` "/Game/Sounds/button.button" 1.0 1.0 0.0 null null))

(event `self.OnReset`)

(fn `SetLightSprites`
  (params (Sprite :type "PaperSprite Object Reference"))
  (`|ExecutionSequence`
    (:`then_0`
      (`PaperSpriteComponent.SetSprite` (`self.PaperSprite3`) Sprite))
    (:`then_1`
      (`PaperSpriteComponent.SetSprite` (`self.PaperSprite1`) Sprite))
    (:`then_2`
      (`PaperSpriteComponent.SetSprite` (`self.PaperSprite2`) Sprite))))

(fn `UserConstructionScript`)