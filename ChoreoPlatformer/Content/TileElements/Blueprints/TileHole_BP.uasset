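; Hole tile that shows a hovering preview of its required item while the inventory holds that item.
; Inventory changes toggle the preview sprite and start a self-restarting timeline that bobs it vertically, with amplitude scaled by the song tempo frequency.
; RefreshState clears the hole by hiding both sprites, ignoring collision, unbinding from the inventory and stopping the hover.
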(event `self.ReceiveBeginPlay`
  (add `InventoryComponent.InventoryChanged` (`DanceUtilsFunctionLibrary.GetInventoryComponent`) (delegate `Toggle Item Preview`))
  (`SceneComponent.SetVisibility` (`self.ItemSprite`) false true))

(event `Toggle Item Preview`
  (`SceneComponent.SetVisibility` (`self.ItemSprite`) (`InventoryComponent.HasItem` (`DanceUtilsFunctionLibrary.GetInventoryComponent`) (`self.RequiredItem`)) true)
  (bind (_direction _hover) (`Timeline|SpriteHover` :!via `PlayFromStart` :!label _label)
    (:`Update`
      (`SceneComponent.K2_SetRelativeLocation` (`self.ItemSprite`) (`KismetMathLibrary.MakeVector` 0.0 0.0 (+ (* _hover (`SongTempoComponent.GetFrequency` (`DanceUtilsFunctionLibrary.GetSongTempoComponent`)) 10.0) 60.0)) false false))
    (:`Finished`
      (`|ExecutionSequence`
        (:`then_0`
          (goto _label :!via `PlayFromStart`))))))

(event `self.RefreshState`
  (`SceneComponent.SetVisibility` (`self.PaperSprite`) false false)
  (`PrimitiveComponent.SetCollisionResponseToAllChannels` (`self.PaperSprite`) "ECR_Ignore")
  (remove `InventoryComponent.InventoryChanged` (`DanceUtilsFunctionLibrary.GetInventoryComponent`) (delegate `Toggle Item Preview`))
  (`SceneComponent.SetVisibility` (`self.ItemSprite`) false true)
  (goto _label :!via `Stop`))

(fn `UserConstructionScript`)