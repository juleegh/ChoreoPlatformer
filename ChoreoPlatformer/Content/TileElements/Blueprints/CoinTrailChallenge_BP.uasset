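; Coin trail challenge tile element that plays out along a row of coins placed on the InterestPoints spline.
; BeginPlay spawns a coin per spline point, giving the first a distinct sprite and the dialog box above it.
; Challenge start and updates hide coins up to CurrentCoin and re-sprite the rest; ending hides all with win or fail feedback.
; The song tempo component's new-tempo event restarts a timeline that bounces every coin's height.
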(event `self.ReceiveBeginPlay`
  (`parent.ReceiveBeginPlay`)
  (`self.SpawnCoins`)
  (add `SongTempoComponent.NewTempoStarted` (`DanceUtilsFunctionLibrary.GetSongTempoComponent`) (delegate `Bounce Coins`)))

(event `self.ChallengeStarted`
  (`GameplayStatics.PlaySound2D` "/Game/Sounds/coin_start.coin_start" 1.0 1.0 0.0 null null :!label _label)
  (`self.UpdateCoins`)
  (`SceneComponent.SetVisibility` (`self.DialogBox`) false true))

(event `Bounce Coins`
  (bind (_direction _height) (`Timeline|Bounce` :!via `PlayFromStart`)
    (:`Update`
      (for _array_element (`self.Coins`)
        (bind _coin (`/Game/TileElements/Blueprints/Coin__BP.Coin` _array_element))
        (bind (_returnvalue_x _returnvalue_y) (`KismetMathLibrary.BreakVector` (`SceneComponent.K2_GetComponentLocation` _coin)))
        (`SceneComponent.K2_SetWorldLocation` _coin (`KismetMathLibrary.MakeVector` _returnvalue_x _returnvalue_y (+ (* _height 10.0) 50.0)) false false)))))

(event `self.ChallengeUpdated`
  (goto _label))

(event `self.ChallengeEnded`
  (params (bWasSuccessful :type Boolean))
  (bind _coins (`self.Coins`))
  (for _array_element (`self.Coins`)
    (`/Game/TileElements/Blueprints/Coin__BP.Toggle` _array_element false))
  (if bWasSuccessful
    (`GameplayStatics.PlaySound2D` "/Game/Sounds/coin_win.coin_win" 1.0 1.0 0.0 null null)
    (`GameplayStatics.SpawnEmitterAtLocation` "/Game/Particles/Stars_PS.Stars_PS" (`SceneComponent.K2_GetComponentLocation` (`/Game/TileElements/Blueprints/Coin__BP.Coin` (`|GetArrayItem` _coins (`KismetArrayLibrary.Array_LastIndex` _coins)))))
    (else
      (`GameplayStatics.PlaySound2D` "/Game/Sounds/coin_fail.coin_fail" 1.0 1.0 0.0 null null))))

(fn `SpawnCoins`
  (for _index (range (`SplineComponent.GetNumberOfSplinePoints` (`self.InterestPoints`)))
    (bind _returnvalue (`|SpawnActorFromClass` "/Game/TileElements/Blueprints/Coin__BP.Coin__BP_C" (`self.GetTransform`) "Undefined" "OverrideRootScale" null null))
    (`KismetArrayLibrary.Array_Add` (`self.Coins`) _returnvalue)
    (`|ExecutionSequence`
      (:`then_0`
        (bind _returnvalue_2 (`SplineComponent.GetLocationAtSplinePoint` (`self.InterestPoints`) _index "World"))
        (`self.K2_SetActorLocation` _returnvalue (+ _returnvalue_2 (0.0 0.0 50.0)) false false))
      (:`then_1`
        (`self.SetActorScale3D` _returnvalue (0.5 0.5 0.5)))
      (:`then_2`
        (if (== _index 0)
          (`/Game/TileElements/Blueprints/Coin__BP.AssignSprite` _returnvalue "/Game/Sprites/challenge_assets_Sprite_11.challenge_assets_Sprite_11")
          (`SceneComponent.K2_SetWorldLocation` (`self.DialogBox`) (+ _returnvalue_2 (0.0 0.0 150.0)) false false)
          (else
            (`/Game/TileElements/Blueprints/Coin__BP.AssignSprite` _returnvalue "/Game/Sprites/challenge_assets_Sprite_13.challenge_assets_Sprite_13")))))))

(fn `UpdateCoins`
  (for (_array_element _array_index) (`self.Coins`)
    (if (<= _array_index (`self.CurrentCoin`))
      (`/Game/TileElements/Blueprints/Coin__BP.Toggle` _array_element false)
      (else
        (`/Game/TileElements/Blueprints/Coin__BP.AssignSprite` _array_element "/Game/Sprites/challenge_assets_Sprite_12.challenge_assets_Sprite_12")))))

(fn `UserConstructionScript`)