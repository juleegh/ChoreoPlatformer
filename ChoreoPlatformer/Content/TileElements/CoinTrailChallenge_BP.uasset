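; Coin trail challenge tile element that places a line of coins along its InterestPoints spline.
; On BeginPlay it spawns a half-scale Coin__BP slightly above each spline point, giving the first coin its own sprite.
; When the challenge starts or updates, it toggles off coins up to CurrentCoin and switches the rest to a third sprite.
; When the challenge ends, it toggles off every coin.
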(event `self.ReceiveBeginPlay`
  (`parent.ReceiveBeginPlay`)
  (`self.SpawnCoins`))

(event `self.ChallengeStarted`
  (`self.UpdateCoins` :!label _label))

(event `self.ChallengeUpdated`
  (goto _label))

(event `self.ChallengeEnded`
  (params (bWasSuccessful :type Boolean))
  (for _array_element (`self.Coins`)
    (`/Game/TileElements/Coin__BP.Toggle` _array_element false)))

(fn `SpawnCoins`
  (for _index (range (`SplineComponent.GetNumberOfSplinePoints` (`self.InterestPoints`)))
    (bind _returnvalue (`|SpawnActorFromClass` "/Game/TileElements/Coin__BP.Coin__BP_C" (`self.GetTransform`) "Undefined" "OverrideRootScale" null null))
    (`KismetArrayLibrary.Array_Add` (`self.Coins`) _returnvalue)
    (`|ExecutionSequence`
      (:`then_0`
        (`self.K2_SetActorLocation` _returnvalue (+ (`SplineComponent.GetLocationAtSplinePoint` (`self.InterestPoints`) _index "World") (0.0 0.0 50.0)) false false))
      (:`then_1`
        (`self.SetActorScale3D` _returnvalue (0.5 0.5 0.5)))
      (:`then_2`
        (if (== _index 0)
          (`/Game/TileElements/Coin__BP.AssignSprite` _returnvalue "/Game/Sprites/challenge_assets_Sprite_4.challenge_assets_Sprite_4")
          (else
            (`/Game/TileElements/Coin__BP.AssignSprite` _returnvalue "/Game/Sprites/challenge_assets_Sprite_6.challenge_assets_Sprite_6")))))))

(fn `UpdateCoins`
  (for (_array_element _array_index) (`self.Coins`)
    (if (<= _array_index (`self.CurrentCoin`))
      (`/Game/TileElements/Coin__BP.Toggle` _array_element false)
      (else
        (`/Game/TileElements/Coin__BP.AssignSprite` _array_element "/Game/Sprites/challenge_assets_Sprite_5.challenge_assets_Sprite_5")))))

(fn `UserConstructionScript`)