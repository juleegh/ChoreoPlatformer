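; Half-coin challenge tile element that marks the start and end of a challenge with two coin sprites.
; On BeginPlay it places both sprites slightly above the first and last points of the InterestPoints spline and makes them visible.
; When the challenge starts, the start coin turns transparent and the end coin swaps its sprite; when the challenge ends, the end coin also turns transparent.
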(event `self.ReceiveBeginPlay`
  (`parent.ReceiveBeginPlay`)
  (`self.SetStartCoin`)
  (`self.SetEndCoin`))

(event `self.ChallengeStarted`
  (`PaperSpriteComponent.SetSprite` (`self.EndCoin`) "/Game/Sprites/challenge_assets_Sprite_1.challenge_assets_Sprite_1")
  (`PaperSpriteComponent.SetSpriteColor` (`self.StartCoin`) (struct :`R` 1.0 :`G` 1.0 :`B` 1.0)))

(event `self.ChallengeEnded`
  (params (bWasSuccessful :type Boolean))
  (`PaperSpriteComponent.SetSpriteColor` (`self.EndCoin`) (struct :`R` 1.0 :`G` 1.0 :`B` 1.0)))

(fn `SetEndCoin`
  (bind _interestpoints (`self.InterestPoints`))
  (`SceneComponent.K2_SetWorldLocation` (`self.EndCoin`) (+ (`SplineComponent.GetLocationAtSplinePoint` _interestpoints (- (`SplineComponent.GetNumberOfSplinePoints` _interestpoints) 1) "World") (0.0 0.0 50.0)) false false)
  (`PaperSpriteComponent.SetSpriteColor` (`self.EndCoin`) (struct :`R` 1.0 :`G` 1.0 :`B` 1.0 :`A` 1.0)))

(fn `SetStartCoin`
  (`SceneComponent.K2_SetWorldLocation` (`self.StartCoin`) (+ (`SplineComponent.GetLocationAtSplinePoint` (`self.InterestPoints`) 0 "World") (0.0 0.0 50.0)) false false)
  (`PaperSpriteComponent.SetSpriteColor` (`self.StartCoin`) (struct :`R` 1.0 :`G` 1.0 :`B` 1.0 :`A` 1.0)))

(fn `UserConstructionScript`)